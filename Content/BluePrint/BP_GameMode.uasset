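; BP_GameMode is a game mode that populates the level with BP_NPC actors when play begins.
; SpawnNPC loops over the configured count, spawning each NPC at a random reachable navigation point around a fixed origin, adjusting for collisions but always spawning.
; OnHumanDeath validates attacker and victim and appears intended to increment a kill count, though its target is unconnected.
; OnPlayerDeath and CheckWinner are empty stubs.
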(event EventBeginPlay
  (CallFunction|SpawnNPC (Variables|Default|GetIn%20Npc%20Spawn%20Count)))

(event EventTick
  (params (DeltaSeconds :type Float%20%28single-precision%29)))

(fn ConstructionScript)

(fn OnHumanDeath
  (params (Attacker :type BP%20Player%20Object%20Reference) (Victim :type BP%20Human%20Object%20Reference))
  (Utilities|IsValid Attacker
    (:Is%20Valid
      (Utilities|IsValid Victim
        (:Is%20Valid
          (Utilities|FlowControl|Sequence
            (:then_0
              ;[0.15 0.15 0.15 0.5] 킬수증가
              (Utilities|IsValid 0
                (:Is%20Valid
                  (Math|Integer|IncrementInt 0))))))))))

(fn SpawnNPC
  (params (InNpcSpawnCount :type Integer))
  (bind (_randomlocation _returnvalue) (AI|Navigation|GetRandomReachablePointinRadius (Math|Vector|MakeVector 0.0 0.0 9e+01) 1e+03 0 0))
  (for _index (range 1 InNpcSpawnCount)
    (if _returnvalue
      (Game|SpawnActorfromClass "/Game/BluePrint/InGame/NPC/BP_NPC.BP_NPC_C" (Math|Transform|MakeTransform _randomlocation "0, 0, 0" "1.000000,1.000000,1.000000") "AdjustIfPossibleButAlwaysSpawn" "MultiplyWithRoot" 0 0))))

(fn OnPlayerDeath)

(fn CheckWinner)