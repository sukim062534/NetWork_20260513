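; BP_Human is a networked human character that can melee-attack other humans and dies when damaged.
; CallAttackHit runs a forward sphere trace on the server and damages every BP_Human it hits, while CallAttackEnd returns the Attack state to IdleMove.
; Damage in either state triggers S2M_Death, which disables movement and capsule collision and ragdolls the mesh.
; The GameMode death notification exists but is unconnected.
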(event Custom|S2M_Death
  (bind _mesh (Variables|Character|GetMesh))
  (Utilities|FlowControl|Sequence
    (:then_0
      (Variables|Default|SetState "NewEnumerator0"))
    (:then_1
      (Pawn|Components|CharacterMovement|DisableMovement (Variables|Character|GetCharacterMovement)))
    (:then_2
      (Collision|SetCollisionEnabled (Variables|Collision|GetCapsuleComponent) "NoCollision"))
    (:then_3
      (Collision|SetCollisionEnabled _mesh "PhysicsOnly")
      (Physics|SetSimulatePhysics _mesh true))))

(event EventBeginPlay)

(event Collision|EventActorBeginOverlap
  (params (OtherActor :type Actor%20Object%20Reference)))

(event EventTick
  (params (DeltaSeconds :type Float%20%28single-precision%29)))

(event Game|Damage|EventAnyDamage
  (params (Damage :type Float%20%28single-precision%29) (DamageType :type Damage%20Type%20Object%20Reference) (InstigatedBy :type Controller%20Object%20Reference) (DamageCauser :type Actor%20Object%20Reference))
  (switch Utilities|FlowControl|Switch|SwitchonEState (Variables|Default|GetState)
    (:NewEnumerator0
      _)
    (:NewEnumerator1
      _))
  (Utilities|FlowControl|Sequence
    (:then_0
      (CallFunction|S2MDeath))))

(event Custom|CallAttackHit
  (bind _returnvalue (Transformation|GetActorLocation))
  ;[0.15 0.15 0.15 0.5] 서버인지 확인
  (Networking|SwitchHasAuthority
    (:Authority
      (bind _outhits (Collision|MultiSphereTraceForObjects _returnvalue (+ _returnvalue (* (Transformation|GetActorForwardVector) (Variables|Default|GetAttack%20Range))) 15.0 (Utilities|Array|MakeArray "ObjectTypeQuery3") false 0 "ForDuration"))
      (for _array_element _outhits
        (bind _asbp_human (Utilities|Casting|CastToBP_Human (.HitActor (Collision|BreakHitResult _array_element))))
        (Game|Damage|ApplyDamage _asbp_human 1.0 0 self)))))

(event Custom|CallAttackEnd
  (switch Utilities|FlowControl|Switch|SwitchonEState (Variables|Default|GetState)
    (:NewEnumerator1
      (Variables|Default|SetState "NewEnumerator0"))))

(fn ConstructionScript)