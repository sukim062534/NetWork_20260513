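; BP_Player is the in-game player Blueprint, handling a state-gated melee or general attack with client-to-server-to-multicast event naming.
; CallAttackInput calls C2S_Attack only in the Idle or Move state, and C2S_Attack repeats that check before calling S2M_Attack.
; S2M_Attack sets State to Attack and plays AM_Attack on the mesh; nothing here restores the state afterward.
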(event Custom|CallAttackInput
  (switch Utilities|FlowControl|Switch|SwitchonEState (Variables|Default|GetState)
    (:NewEnumerator0
      (CallFunction|C2SAttack))))

(event Custom|C2S_Attack
  (switch Utilities|FlowControl|Switch|SwitchonEState (Variables|Default|GetState)
    (:NewEnumerator0
      (CallFunction|S2MAttack))))

(event Custom|S2M_Attack
  (Utilities|FlowControl|Sequence
    (:then_0
      (Variables|Default|SetState "NewEnumerator1"))
    (:then_1
      (Animation|Montage|PlayMontage (Variables|Character|GetMesh) "/Game/Animation/AM_Attack.AM_Attack"))))

(fn ConstructionScript
  (|CallParentFunction))