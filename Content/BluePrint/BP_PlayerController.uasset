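; Player controller that turns Enhanced Input actions into look, movement, jump, crouch and attack commands for BP_Player.
; On BeginPlay it caches the controlled BP_Player and adds the IMC_Default mapping context.
; Look feeds yaw and pitch input, while movement follows the control rotation with pitch zeroed.
; Jump and crouch call the character's built-in functions; attack calls CallAttackInput on both Started and Triggered.
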(event Input|EnhancedActionEvents|EnhancedInputActionIA_Look
  (params (ActionValue :type Vector%202D%20Structure) (ElapsedSeconds :type Float%20%28double-precision%29) (TriggeredSeconds :type Float%20%28double-precision%29) (InputAction :type Input%20Action%20Object%20Reference :default "/Game/Input/IA_Look.IA_Look"))
  (bind (_x _y) (Math|Vector2D|BreakVector2D ActionValue))
  (Class|PlayerController|AddYawInput _x)
  (Class|PlayerController|AddPitchInput _y))

(event Input|EnhancedActionEvents|EnhancedInputActionIA_Move
  (params (ActionValue :type Vector%202D%20Structure) (ElapsedSeconds :type Float%20%28double-precision%29) (TriggeredSeconds :type Float%20%28double-precision%29) (InputAction :type Input%20Action%20Object%20Reference :default "/Game/Input/IA_Move.IA_Move"))
  (bind _returnvalue (Pawn|GetControlRotation :!class /Script/Engine.Controller))
  (bind _returnvalue_2 (Pawn|GetControlRotation :!class /Script/Engine.Controller))
  (Pawn|Input|AddMovementInput (Variables|Default|GetAs%20BP%20Player) (Math|Vector|GetRightVector (Math|Rotator|MakeRotator (.roll _returnvalue_2) 0.0 (.yaw _returnvalue_2))) (.x ActionValue) false)
  (Pawn|Input|AddMovementInput (Variables|Default|GetAs%20BP%20Player) (Math|Vector|GetForwardVector (Math|Rotator|MakeRotator (.roll _returnvalue) 0.0 (.yaw _returnvalue))) (.y ActionValue) false))

(event Input|EnhancedActionEvents|EnhancedInputActionIA_Jump
  (params (ActionValue :type Boolean) (ElapsedSeconds :type Float%20%28double-precision%29) (TriggeredSeconds :type Float%20%28double-precision%29) (InputAction :type Input%20Action%20Object%20Reference :default "/Game/Input/IA_Jump.IA_Jump"))
  (bind _as_bp_player (Variables|Default|GetAs%20BP%20Player))
  (:Started
    (Character|Jump _as_bp_player))
  (:Canceled
    (Character|StopJumping _as_bp_player)))

(event Input|EnhancedActionEvents|EnhancedInputActionIA_Attack
  (params (ActionValue :type Boolean) (ElapsedSeconds :type Float%20%28double-precision%29) (TriggeredSeconds :type Float%20%28double-precision%29) (InputAction :type Input%20Action%20Object%20Reference :default "/Game/Input/IA_Attack.IA_Attack"))
  (:Triggered
    (Default|CallAttackInput (Variables|Default|GetAs%20BP%20Player) :!label _label))
  (:Started
    (goto _label)))

(event Input|EnhancedActionEvents|EnhancedInputActionIA_Crouch
  (params (ActionValue :type Boolean) (ElapsedSeconds :type Float%20%28double-precision%29) (TriggeredSeconds :type Float%20%28double-precision%29) (InputAction :type Input%20Action%20Object%20Reference :default "/Game/Input/IA_Crouch.IA_Crouch"))
  (bind _as_bp_player (Variables|Default|GetAs%20BP%20Player))
  (:Started
    (Character|Crouch _as_bp_player))
  (:Completed
    (Character|UnCrouch _as_bp_player)))

(event EventBeginPlay
  (bind _self self)
  (bind _returnvalue (PlayerController|LocalPlayerSubsystems|GetEnhancedInputLocalPlayerSubsystem _self))
  (bind _asbp_player (Utilities|Casting|CastToBP_Player (Pawn|GetControlledPawn)))
  (Variables|Default|SetAs%20BP%20Player _asbp_player)
  (Utilities|IsValid _returnvalue
    (:Is%20Valid
      (Input|AddMappingContext _returnvalue "/Game/Input/IMC_Default.IMC_Default" 0 "(bIgnoreAllPressedKeysUntilRelease=True,bForceImmediately=False,bNotifyUserSettings=False)"))))

(event EventTick
  (params (DeltaSeconds :type Float%20%28single-precision%29)))

(fn ConstructionScript)